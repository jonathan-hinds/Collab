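; BP_ItemBase is a base item pickup that adds itself to the player's inventory when interacted with.
; BeginPlay applies the mesh from ItemData to ItemMesh.
; Interact passes ItemData and its quantity to the third-person character's InventoryComponent, then destroys the actor after a short delay.
; Unconnected logic, which never runs, would uniformly scale the mesh to fit BoundingBox when ScaleToBounds is set.
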(event `self.ReceiveBeginPlay`
  (`StaticMeshComponent.SetStaticMesh` (`self.ItemMesh`) (`/Game/Inventory/DA_ItemBase.Mesh` (`self.ItemData`))))

(event `/Game/Interaction/BPI_Interactable.Interact`
  (params (InteractActor :type "Actor Object Reference"))
  (bind _itemdata (`self.ItemData`))
  (bind _asbp_third_person_character (cast `/Game/ThirdPerson/Blueprints/BP_ThirdPersonCharacter` (`GameplayStatics.GetPlayerPawn` 0)))
  (`/Game/Components/InventoryComponent.AddItem` (`/Game/ThirdPerson/Blueprints/BP_ThirdPersonCharacter.InventoryComponent` _asbp_third_person_character) _itemdata (`/Game/Inventory/DA_ItemBase.Quantity` _itemdata))
  (`KismetSystemLibrary.Delay` 0.2)
  (`self.K2_DestroyActor`))

(fn `UserConstructionScript`)